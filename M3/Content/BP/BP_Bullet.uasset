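; BP_Bullet is a projectile that flies along the player pawn's forward direction and detects hits on BP_Turret actors.
; BeginPlay caches a fixed step vector, which Tick adds to the Sphere's location each frame without sweep or delta-time scaling.
; Tick scans all turrets by position tolerance, destroying only the bullet and playing a hit sound at world origin on a match.
; It also destroys itself when out of range of the player.
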(event `self.ReceiveBeginPlay`
  (bind _output_get (set `self.Rot` (* (`KismetMathLibrary.Conv_RotatorToVector` (`self.K2_GetActorRotation` (`GameplayStatics.GetPlayerPawn` 0))) 50))))

(event `self.ReceiveTick`
  (params (DeltaSeconds :type "Float (single-precision)"))
  (bind _returnvalue (`SceneComponent.K2_GetComponentLocation` (`self.Sphere`)))
  (if (== (`self.K2_GetActorLocation` (`GameplayStatics.GetPlayerPawn` 0)) _returnvalue :`ErrorTolerance` 12000.0)
    (`self.K2_SetActorLocation` (+ _returnvalue (stale `self.ReceiveBeginPlay` _output_get)))
    (bind _outactors (`GameplayStatics.GetAllActorsOfClass` "/Game/BP/BP_Turret.BP_Turret_C"))
    (for _array_element _outactors
      (if (== (`self.K2_GetActorLocation` _array_element) (`self.K2_GetActorLocation`) :`ErrorTolerance` 150.0)
        (`self.K2_DestroyActor`)
        (`GameplayStatics.PlaySoundAtLocation` "/Game/Sound/Cue_Hit.Cue_Hit" (0.0 0.0 0.0) (struct) 1.0 1.0 0.0 null null null)))
    (else
      (`self.K2_DestroyActor`))))

(fn `UserConstructionScript`)