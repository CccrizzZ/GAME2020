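; BP_Turret is a turret actor that tracks the player pawn and fires BP_TBullet projectiles at intervals.
; Tick spins the Barrel continuously and, while the player is within range, turns the Head to face them.
; A Delay inside Tick paces the shots, each spawning a bullet just above the Barrel and calling Launch with the Barrel's location.
; Each shot plays the Fire sound at the world origin.
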(event `self.ReceiveTick`
  (params (DeltaSeconds :type "Float (single-precision)"))
  (bind _returnvalue (`self.K2_GetActorLocation`))
  (bind _returnvalue_2 (`SceneComponent.K2_GetComponentLocation` (`self.Barrel`)))
  (bind _returnvalue_3 (`self.K2_GetActorLocation` (`GameplayStatics.GetPlayerPawn` 0)))
  (`SceneComponent.K2_AddLocalRotation` (`self.Barrel`) (`KismetMathLibrary.MakeRotator` 0.0 0.0 (* DeltaSeconds 200.0)) false false)
  (if (== _returnvalue _returnvalue_3 :`ErrorTolerance` 5000.0)
    (`SceneComponent.K2_SetRelativeRotation` (`self.Head`) (`KismetMathLibrary.FindLookAtRotation` _returnvalue _returnvalue_3) false false)
    (`KismetSystemLibrary.Delay` 3.0)
    (bind _returnvalue_4 (`|SpawnActorFromClass` "/Game/BP/BP_TBullet.BP_TBullet_C" (`KismetMathLibrary.Conv_VectorToTransform` (+ _returnvalue_2 (0.0 0.0 15.0))) "AlwaysSpawn" "OverrideRootScale" null null))
    (bind _output_get (set `self.Bullet` _returnvalue_4))
    (`/Game/BP/BP_TBullet.Launch` _output_get _returnvalue_2)
    (`GameplayStatics.PlaySoundAtLocation` "/Game/Sound/fire.fire" (0.0 0.0 0.0) (struct) 1.0 1.0 0.0 null null null)))

(fn `UserConstructionScript`)