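; Player projectile Blueprint that flies along the player pawn's facing direction and destroys BP_Turret actors it hits.
; BeginPlay caches a fixed step from the pawn's forward vector, and Tick adds it to the Sphere's location without sweep or delta-time scaling.
; Each tick destroys overlapping turrets within a tolerance and plays a hit sound.
; The bullet survives hits and destroys itself once out of range of the player.
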(event `self.ReceiveBeginPlay`
  (bind _output_get (set `self.Rot` (* (`KismetMathLibrary.Conv_RotatorToVector` (`self.K2_GetActorRotation` (`GameplayStatics.GetPlayerPawn` 0))) 50))))

(event `self.ReceiveTick`
  (params (DeltaSeconds :type "Float (single-precision)"))
  (bind _returnvalue (`self.K2_GetActorLocation`))
  (bind _returnvalue_2 (`SceneComponent.K2_GetComponentLocation` (`self.Sphere`)))
  (if (== (`self.K2_GetActorLocation` (`GameplayStatics.GetPlayerPawn` 0)) _returnvalue_2 :`ErrorTolerance` 6000.0)
    (`self.K2_SetActorLocation` (+ _returnvalue_2 (stale `self.ReceiveBeginPlay` _output_get)))
    (for _array_element (`self.GetOverlappingActors` self "/Game/BP/BP_Turret.BP_Turret_C")
      (bind _output_get (set `self.actorRef` _array_element))
      (if (== (`self.K2_GetActorLocation` _array_element) _returnvalue :`ErrorTolerance` 300.0)
        (`self.K2_DestroyActor` _output_get)
        (`GameplayStatics.PlaySoundAtLocation` "/Game/Sound/Cue_Hit.Cue_Hit" _returnvalue (struct) 1.0 1.0 0.0 null null null)))
    (else
      (`self.K2_DestroyActor`))))

(fn `UserConstructionScript`)