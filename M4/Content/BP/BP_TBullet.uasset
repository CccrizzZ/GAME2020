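; BP_TBullet is a projectile actor fired toward the player that registers a hit by proximity.
; Launch stores a fixed step vector from the parent location toward player pawn 0, so it does not home.
; Tick teleports it by that step without sweep or delta-time scaling, destroying it beyond range of the parent location.
; Coming near the player destroys it and plays a hit sound at the world origin, with no damage applied.
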(event `self.ReceiveTick`
  (params (DeltaSeconds :type "Float (single-precision)"))
  (if (== (`self.K2_GetActorLocation`) (stale `Launch` ParentLocation) :`ErrorTolerance` 5000.0)
    (`self.K2_SetActorLocation` (+ (stale `Launch` _output_get) (`SceneComponent.K2_GetComponentLocation` (`self.Sphere`))))
    (if (== (`SceneComponent.K2_GetComponentLocation` (`self.Sphere`)) (`self.K2_GetActorLocation` (`GameplayStatics.GetPlayerPawn` 0)) :`ErrorTolerance` 150.0)
      (`self.K2_DestroyActor`)
      (`GameplayStatics.PlaySoundAtLocation` "/Game/Sound/isHit.isHit" (0.0 0.0 0.0) (struct) 1.0 1.0 0.0 null null null))
    (else
      (`self.K2_DestroyActor`))))

(event `Launch`
  (params (ParentLocation :type "Vector Structure"))
  (bind _output_get (set `self.rot` (* (`KismetMathLibrary.Conv_RotatorToVector` (`KismetMathLibrary.FindLookAtRotation` ParentLocation (`self.K2_GetActorLocation` (`GameplayStatics.GetPlayerPawn` 0)))) 50))))

(fn `UserConstructionScript`)