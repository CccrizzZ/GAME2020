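; BP_Turret is a destructible turret that fires at the player pawn when within horizontal and vertical range.
; Tick spins the barrel, turns a health-scaled plane toward the player and, in range, aims the head.
; A Delay inside Tick paces firing: it spawns and launches a BP_TBullet, flashes a light and plays a sound at world origin.
; DecreaseHP subtracts fixed damage and destroys the actor at zero.
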(event `self.ReceiveTick`
  (params (DeltaSeconds :type "Float (single-precision)"))
  (bind (_returnvalue_x _returnvalue_y _returnvalue_z) (`KismetMathLibrary.BreakVector` (`self.K2_GetActorLocation`)))
  (bind _returnvalue (`GameplayStatics.GetPlayerPawn` 0))
  (bind _pointlight1 (`self.PointLight1`))
  (bind (_returnvalue_x_2 _returnvalue_y_2 _returnvalue_z_2) (`KismetMathLibrary.BreakVector` (`self.K2_GetActorLocation` _returnvalue)))
  (bind _returnvalue_2 (`SceneComponent.K2_GetComponentLocation` (`self.Barrel`)))
  (bind (_returnvalue_roll _returnvalue_pitch _returnvalue_yaw) (`KismetMathLibrary.BreakRotator` (`KismetMathLibrary.FindLookAtRotation` (`self.K2_GetActorLocation`) (`self.K2_GetActorLocation` (`GameplayStatics.GetPlayerPawn` 0)))))
  ;[1 1 1] Tick
  (`SceneComponent.SetRelativeScale3D` (`self.Plane`) (`KismetMathLibrary.MakeVector` 0.25 (/ (`KismetMathLibrary.Conv_IntToDouble` (`self.HPval`)) 50.0)))
  (`SceneComponent.K2_SetRelativeRotation` (`self.Plane`) (`KismetMathLibrary.MakeRotator` 0.0 (- _returnvalue_pitch 90.0) _returnvalue_yaw) false false)
  (`SceneComponent.K2_AddLocalRotation` (`self.Barrel`) (`KismetMathLibrary.MakeRotator` 0.0 0.0 (* DeltaSeconds 200.0)) false false)
  (if (and (== (`KismetMathLibrary.MakeVector` 0.0 0.0 _returnvalue_z) (`KismetMathLibrary.MakeVector` 0.0 0.0 _returnvalue_z_2) :`ErrorTolerance` 300.0) (== (`KismetMathLibrary.MakeVector` _returnvalue_x _returnvalue_y) (`KismetMathLibrary.MakeVector` _returnvalue_x_2 _returnvalue_y_2) :`ErrorTolerance` 5000.0))
    (`SceneComponent.K2_SetRelativeRotation` (`self.Head`) (`KismetMathLibrary.FindLookAtRotation` (`self.K2_GetActorLocation`) (`self.K2_GetActorLocation` _returnvalue)) false false)
    (`KismetSystemLibrary.Delay` 3.0)
    (bind _returnvalue_3 (`|SpawnActorFromClass` "/Game/BP/BP_TBullet.BP_TBullet_C" (`KismetMathLibrary.Conv_VectorToTransform` (+ _returnvalue_2 (0.0 0.0 15.0))) "AlwaysSpawn" "OverrideRootScale" null null))
    (bind _output_get (set `self.Bullet` _returnvalue_3))
    (`/Game/BP/BP_TBullet.Launch` _output_get _returnvalue_2)
    (`SceneComponent.SetVisibility` _pointlight1 true false)
    (`KismetSystemLibrary.Delay` 0.2)
    (`SceneComponent.SetVisibility` _pointlight1 false false)
    (`GameplayStatics.PlaySoundAtLocation` "/Game/Sound/fire.fire" (0.0 0.0 0.0) (struct) 1.0 1.0 0.0 null null null)))

(event `DecreaseHP`
  (bind _hpval (`self.HPval`))
  ;[1 1 1] Decrease HP
  (set `self.HPval` (- _hpval 20))
  (if (<= _hpval 0)
    (`self.K2_DestroyActor`)))

(fn `UserConstructionScript`)